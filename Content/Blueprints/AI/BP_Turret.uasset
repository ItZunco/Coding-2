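; AI turret that turns to face a sighted target and fires bullets at it.
; HandleSight stores the target and starts Tracking, which enables per-tick look-at rotation.
; Tracking and Attacking call each other in a one-second loop, spawning BP_Bullet at ProjectileSpawn with a forward impulse.
; Losing sight clears TrackingTarget, but the loop has no exit check, so it re-enables tracking and keeps firing.
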(event Custom|FireProjectile
  (bind _projectilespawn (Variables|Default|GetProjectileSpawn))
  (bind _returnvalue (Game|SpawnActorfromClass "/Game/Blueprints/AI/BP_Bullet.BP_Bullet_C" (Transformation|GetWorldTransform _projectilespawn) "Undefined" "MultiplyWithRoot" 0 0))
  (Physics|AddImpulse (Variables|/Game/Blueprints/AI/BP_Bullet.BP_Bullet_C|GetSphere _returnvalue) (* (Math|Vector|GetForwardVector _projectilespawn) 3e+03) "None" false))

(event Custom|HandleSight
  (params (Target :type Actor%20Object%20Reference) (SuccessfulSense :type Boolean))
  (if SuccessfulSense
    (Variables|Default|SetTarget Target)
    (CallFunction|Tracking)
    (else
      (CallFunction|Looking))))

(event Custom|Looking
  (Variables|Default|SetTrackingTarget false))

(event Custom|Tracking
  (Variables|Default|SetTrackingTarget true)
  (Utilities|FlowControl|Delay 1.0)
  (CallFunction|Attacking))

(event Custom|Attacking
  (CallFunction|FireProjectile)
  (CallFunction|Tracking))

(event EventTick
  (params (DeltaSeconds :type Float%20%28single-precision%29))
  (if (Variables|Default|GetTrackingTarget)
    (Transformation|SetActorRotation (Math|Rotator|FindLookatRotation (Transformation|GetActorLocation) (Transformation|GetActorLocation (Variables|Default|GetTarget))))))

(fn ConstructionScript)