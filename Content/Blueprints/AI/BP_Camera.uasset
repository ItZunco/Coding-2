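; BP_Camera is an AI security camera that raises an alarm when its sight senses a target.
; HandleSight turns the mesh green, plays a sound at the camera and calls CheckAlarm with the stimulus location on every BP_SomeRandomDude in the level.
; When the target is lost, it only prints a message and turns the mesh red.
; The event graph is empty, and nothing in this file calls HandleSight.
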(event EventBeginPlay)

(event Collision|EventActorBeginOverlap
  (params (OtherActor :type Actor%20Object%20Reference)))

(event EventTick
  (params (DeltaSeconds :type Float%20%28single-precision%29)))

(fn ConstructionScript)

(fn HandleSight
  (params (TargetActor :type Actor%20Object%20Reference) (StimulusLocation :type Vector) (SuccessfullySensed :type Boolean))
  (bind _staticmesh (Variables|Default|GetStaticMesh))
  (if SuccessfullySensed
    (Development|PrintText "Aquired Target")
    (Rendering|Material|SetMaterial _staticmesh 0 "/AnimationSharing/AnimSharingGreen.AnimSharingGreen")
    (Audio|PlaySoundatLocation "/Engine/EditorSounds/Notifications/CompileFailed_Cue.CompileFailed_Cue" (Transformation|GetActorLocation) "0, 0, 0" 1.0 1.0 0.0 "/Game/Audio/Attenuation.Attenuation" 0 0 0)
    (bind _outactors (Actor|GetAllActorsOfClass "/Game/Blueprints/AI/BP_SomeRandomDude.BP_SomeRandomDude_C"))
    (for _array_element _outactors
      (Default|CheckAlarm _array_element StimulusLocation))
    (else
      (Development|PrintText "Lost Target")
      (Rendering|Material|SetMaterial _staticmesh 0 "/AnimationSharing/AnimSharingRed.AnimSharingRed"))))