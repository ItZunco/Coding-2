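; StateTree task that picks a random wander destination for an AI character.
; On entering the state, it queries the navmesh for a reachable-area point within Radius of Origin and stores it in RandomLocation.
; An Origin near zero is first replaced by the capsule's forward vector, a unit direction rather than the character's location.
; The task itself neither moves the character nor calls Finish Task.
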(event EventLatentEnterState
  (params (Transition :type State%20Tree%20Transition%20Result%20Structure%20%28by%20ref%29))
  (if (Utilities|Operators|EqualEqual :A (Variables|Default|GetOrigin) :ErrorTolerance 0.1)
    (Variables|Default|SetOrigin (Math|Vector|GetForwardVector (Variables|/Script/Engine.Character|GetCapsuleComponent (Variables|Context|GetCharacter)))))
  (bind _randomlocation (Class|NavigationSystemV1|GetRandomLocationinNavigableRadius (Variables|Default|GetOrigin) (Variables|Default|GetRadius) 0 0))
  (Variables|Default|SetRandom%20Location _randomlocation))