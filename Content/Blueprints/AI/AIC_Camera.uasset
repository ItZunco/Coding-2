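; AI controller for security cameras and turrets that relays perception updates to whichever of the two it possesses.
; On possession it caches the pawn as BP_Camera or BP_Turret.
; Perception updates from actors without the "AI" tag print a debug message, then pass through HandleSight to that pawn's own HandleSight.
; Disconnected leftover nodes for material swaps, sound and alarm checks never run.
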(event OnTargetPerceptionUpdated(AIPerception)
  (params (Actor :type Actor%20Object%20Reference) (Stimulus :type AI%20Stimulus%20Structure))
  (bind (_age _expirationage _strength _stimuluslocation _receiverlocation _tag _bsuccessfullysensed) (Utilities|Struct|BreakAIStimulus Stimulus))
  (if (not (Actor|ActorHasTag Actor "AI"))
    (bind _returnvalue (Class|AIPerceptionSystem|GetSenseClassforStimulus Stimulus))
    (Development|PrintText (Utilities|Text|FormatText "Sensed: {actor} with {name} 
Tag: {tag}" Actor (Utilities|GetClassDisplayName _returnvalue) _tag))
    (switch name _tag
      (:Default
        (switch string (Utilities|GetClassDisplayName _returnvalue)
          (:Default
            (CallFunction|HandleSight Actor _stimuluslocation _bsuccessfullysensed)))))))

(event EventBeginPlay)

(event EventTick
  (params (DeltaSeconds :type Float%20%28single-precision%29)))

(event EventPossess
  (params (PossessedPawn :type Pawn%20Object%20Reference))
  (bind _asbp_camera (Utilities|Casting|CastToBP_Camera PossessedPawn)
    (:then
      (Variables|Default|SetAs%20BP%20Camera _asbp_camera))
    (:CastFailed
      (bind _asbp_turret (Utilities|Casting|CastToBP_Turret PossessedPawn))
      (Variables|Default|SetAs%20BP%20Turret _asbp_turret))))

(fn ConstructionScript)

(fn HandleSight
  (params (TargetActor :type Actor%20Object%20Reference) (StimulusLocation :type Vector) (SuccessfullySensed :type Boolean))
  (bind _as_bp_camera (Variables|Default|GetAs%20BP%20Camera)
    (:then
      (Default|HandleSight _as_bp_camera TargetActor StimulusLocation SuccessfullySensed))
    (:else
      (bind _as_bp_turret (Variables|Default|GetAs%20BP%20Turret)
        (:then
          (Default|HandleSight _as_bp_turret TargetActor SuccessfullySensed))
        (:else)))))