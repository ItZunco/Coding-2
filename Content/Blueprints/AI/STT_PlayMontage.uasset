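; StateTree task that plays a montage on the AI character and deals a small amount of damage to whatever is in front of it.
; On state entry it starts the montage and immediately runs a short forward sphere trace, applying damage to the hit actor.
; Montage completion finishes the task as succeeded and interruption as failed.
; Montage notifies only print text and do not time the hit.
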(event EventLatentEnterState
  (params (Transition :type State%20Tree%20Transition%20Result%20Structure%20%28by%20ref%29))
  (bind _character (Variables|Context|GetCharacter))
  (bind _returnvalue (Transformation|GetActorLocation _character))
  (bind _notifyname (Animation|Montage|PlayMontage (Variables|/Script/Engine.Character|GetMesh _character) (Variables|Default|GetMontage%20to%20Play))
    (:then
      (bind (_outhit _returnvalue_2) (Collision|SphereTraceByChannel _returnvalue (+ _returnvalue (* (Math|Vector|GetForwardVector (Variables|/Script/Engine.Character|GetCapsuleComponent _character)) 1.5e+02)) 0.0 "TraceTypeQuery1" false (Utilities|Array|MakeArray (Variables|Context|GetCharacter)) "None"))
      (if _returnvalue_2
        (Game|Damage|ApplyDamage (.HitActor (Collision|BreakHitResult _outhit)) 0.2 (AI|GetAIController 0) (Variables|Context|GetCharacter))))
    (:OnCompleted
      (StateTree|FinishTask true))
    (:OnInterrupted
      (StateTree|FinishTask false))
    (:OnNotifyBegin
      (Development|PrintText (Utilities|Text|FormatText (Utilities|Text|ToText(Name) _notifyname))))))