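; BP_EnemyMel is an AI-controlled enemy that tracks its own health and is destroyed when it runs out.
; On BeginPlay it caches its AIC_Base controller.
; Any damage is reported to AI perception, sent to the controller's StateTree as a TookDamage event, then subtracted from health.
; The GetHealth event, despite its name, adds health and clamps it to a normalized zero-to-one range.
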(event Custom|GetHealth
  (params (AddHealth :type Float%20%28double-precision%29))
  (Variables|Default|SetHealth (Math|Float|Clamp(Float) (+ (Variables|Default|GetHealth) AddHealth))))

(event EventBeginPlay
  (bind _asaic_base (Utilities|Casting|CastToAIC_Base (Pawn|GetController)))
  (Variables|Default|SetAIC _asaic_base))

(event Collision|EventActorBeginOverlap
  (params (OtherActor :type Actor%20Object%20Reference)))

(event EventTick
  (params (DeltaSeconds :type Float%20%28single-precision%29)))

(event Game|Damage|EventAnyDamage
  (params (Damage :type Float%20%28single-precision%29) (DamageType :type Damage%20Type%20Object%20Reference) (InstigatedBy :type Controller%20Object%20Reference) (DamageCauser :type Actor%20Object%20Reference))
  (Class|AISenseDamage|ReportDamageEvent self InstigatedBy Damage (Transformation|GetActorLocation) "0, 0, 0" "None")
  (Gameplay|StateTree|SendStateTreeEvent (Variables|/Game/Blueprints/AI/AIC_Base.AIC_Base_C|GetStateTreeAI (Variables|Default|GetAIC)) (Utilities|Struct|MakeStateTreeEvent "(TagName=\"Ai.Event.TookDamage\")") :!class /Script/GameplayStateTreeModule.StateTreeComponent)
  (bind _output_get (Variables|Default|SetHealth (- (Variables|Default|GetHealth) Damage)))
  (if (not (> _output_get 0.0))
    (Development|PrintText "Enemy Defeated")
    (Actor|DestroyActor)))

(fn ConstructionScript)