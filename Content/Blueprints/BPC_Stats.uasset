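; BPC_Stats is a Blueprint component that holds a character's stats struct: health, energy, boost, cash, experience and save location.
; GetCanSprint allows sprinting while boost is above a small threshold, and Sprintng subtracts a given amount from boost without clamping.
; Every Tick, DebugStats prints health, energy, boost and experience as on-screen text with zero duration, giving a live readout.
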(event Custom|DebugStats
  (params (Duration :type Float%20%28double-precision%29))
  (bind _stats (Variables|Default|GetStats))
  (bind (_health _energy _boost _cash _experience) (Utilities|Struct|BreakS_Stats _stats))
  (Development|PrintText (Utilities|Text|FormatText "HP: {Health}, EP: {Energy}, Boost: {Boost}, EXP: {Experience}" _health _energy _boost _experience) true true (Utilities|Struct|MakeLinearColor 1.0 0.0 0.1 1.0) Duration))

(event EventBeginPlay)

(event EventTick
  (params (DeltaSeconds :type Float%20%28single-precision%29))
  (CallFunction|DebugStats 0.0))

(fn GetCanSprint
  (return (> (.boost (Variables|Default|GetStats)) 0.1)))

(fn Sprintng
  (params (Reduce%20Boost%20By :type Float%20%28double-precision%29))
  (Variables|Default|SetStats (Utilities|Struct|MakeS_Stats (.health (Variables|Default|GetStats)) (.energy (Variables|Default|GetStats)) (- (.boost (Variables|Default|GetStats)) Reduce%20Boost%20By) (.cash (Variables|Default|GetStats)) (.experience (Variables|Default|GetStats)) (.savelocation (Variables|Default|GetStats)))))