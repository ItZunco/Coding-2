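; Chest actor that opens a storage menu when the first-person player walks into its sphere.
; It creates a W_ChestMenu bound to its BPCInventory component at BeginPlay, then shows it alongside the player's inventory on overlap.
; Overlap also adds the chest inventory to GM_SaveLoad's LevelState, and LoadInventory writes a supplied EnumInv back into the component.
; Leaving the sphere removes only the chest menu.
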(event OnComponentBeginOverlap(Sphere)
  (params (OverlappedComponent :type Primitive%20Component%20Object%20Reference) (OtherActor :type Actor%20Object%20Reference) (OtherComp :type Primitive%20Component%20Object%20Reference) (OtherBodyIndex :type Integer) (bFromSweep :type Boolean) (SweepResult :type Hit%20Result%20Structure%20%28by%20ref%29))
  (bind _asbp_first_person_character (Utilities|Casting|CastToBP_FirstPersonCharacter OtherActor))
  (UserInterface|Viewport|AddtoViewport (stale EventBeginPlay _returnvalue) 0) ; show shop keep inventory
  (Default|ShowInventory _asbp_first_person_character) ; Show player inventory
  (bind _asgm_save_load (Utilities|Casting|CastToGM_SaveLoad (Game|GetGameMode)))
  (Default|AddInventory (Variables|/Game/Blueprints/SaveLoad/GM_SaveLoad.GM_SaveLoad_C|GetLevel%20State _asgm_save_load) (Variables|Default|GetBPC_Inventory)))

(event OnComponentEndOverlap(Sphere)
  (params (OverlappedComponent :type Primitive%20Component%20Object%20Reference) (OtherActor :type Actor%20Object%20Reference) (OtherComp :type Primitive%20Component%20Object%20Reference) (OtherBodyIndex :type Integer))
  (Utilities|Casting|CastToBP_FirstPersonCharacter OtherActor)
  (Widget|RemovefromParent (stale EventBeginPlay _returnvalue)))

(event Custom|Load%20Inventory
  (params (EnumInv :type Array%20of%20E_Item%20Enums :default "NewEnumerator0"))
  (Variables|/Game/Blueprints/BPC_Inventory.BPC_Inventory_C|SetEnumInv (Variables|Default|GetBPC_Inventory) EnumInv))

(event EventBeginPlay
  (bind _returnvalue (UserInterface|CreateWidget "/Game/UI/W_ChestMenu.W_ChestMenu_C" 0 (Variables|Default|GetBPC_Inventory))))

(fn ConstructionScript)