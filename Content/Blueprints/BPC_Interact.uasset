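; Interaction component for the first-person character that handles looking at, picking up, dropping, using and swapping held items.
; A self-repeating delayed sphere trace from the camera tracks the last BPI_Item actor in view and shows a pickup prompt.
; Picked-up items attach to the hand and are recorded in the inventory belt, refreshing its grid.
; Slot swaps and active-slot updates destroy the held actor and spawn the slot's Blueprint in its place.
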(event Custom|Looking
  (bind _first_person_camera (Variables|Default|GetFirst%20Person%20Camera))
  (bind _returnvalue (Transformation|GetWorldLocation _first_person_camera))
  (Utilities|FlowControl|Delay (Variables|Default|GetInteractInterval))
  (bind (_outhit _returnvalue_2) (Collision|SphereTraceByChannel _returnvalue (+ _returnvalue (* (Math|Vector|GetForwardVector _first_person_camera) (Variables|Default|GetLookDistance))) 2e+01 "TraceTypeQuery1" false 0 "None" true "(R=1.000000,G=0.023057,B=0.071149,A=1.000000)" "(R=0.029093,G=1.000000,B=0.143793,A=1.000000)" 1.0))
  (if _returnvalue_2
    (if (Utilities|DoesObjectImplementInterface (.HitActor (Collision|BreakHitResult _outhit)) "/Game/Blueprints/BPI_Item.BPI_Item_C")
      (Variables|Default|SetLast%20Touched%20Item (.HitActor (Collision|BreakHitResult _outhit)))
      (Development|PrintText (Utilities|Text|FormatText "Press E to pick up {name}" (Utilities|GetDisplayName (.HitActor (Collision|BreakHitResult _outhit)))) true true "(R=0.000000,G=0.660000,B=1.000000,A=1.000000)" (Variables|Default|GetInteractInterval))
      (else
        (Variables|Default|SetLast%20Touched%20Item 0)))
    (else
      (Variables|Default|SetLast%20Touched%20Item 0)))
  (CallFunction|Looking))

(event Custom|Pick%20Up
  (bind _player (Variables|Default|GetPlayer))
  (Variables|Default|GetHeldItem
    (:then
      (Development|PrintText "We're already holding something" true true "(R=1.000000,G=0.075243,B=0.056461,A=1.000000)"))
    (:else
      (bind _last_touched_item (Variables|Default|GetLast%20Touched%20Item)
        (:then
          (bind _item_type (Class|BPIItem|Pickup(Message) _last_touched_item self))
          (Transformation|AttachComponentToComponent _last_touched_item (Variables|/Game/FirstPerson/Blueprints/BP_FirstPersonCharacter.BP_FirstPersonCharacter_C|GetHandHoldPoint (Variables|Default|GetPlayer)) "None" "SnapToTarget" "SnapToTarget" "KeepRelative" true)
          (Variables|Default|SetHeldItem _last_touched_item)
          (Variables|Default|SetLast%20Touched%20Item 0)
          (Default|SetSlot (Variables|/Game/FirstPerson/Blueprints/BP_FirstPersonCharacter.BP_FirstPersonCharacter_C|GetBPC_Inv_Belt _player) _item_type (Variables|Default|GetActive%20Slot))
          (Default|RefreshGrid (Variables|/Game/UI/W_Belt.W_Belt_C|GetW_InventoryGrid_0 (Variables|/Game/FirstPerson/Blueprints/BP_FirstPersonCharacter.BP_FirstPersonCharacter_C|GetBelt%20Widget _player))))
        (:else
          (Development|PrintText "We're not looking at anything" true true "(R=1.000000,G=0.075243,B=0.056461,A=1.000000)"))))))

(event Custom|SwapItem
  (params (New%20Slot :type Integer))
  (bind _player (Variables|Default|GetPlayer))
  (bind _player_2 (Variables|Default|GetPlayer))
  (bind _handholdpoint (Variables|/Game/FirstPerson/Blueprints/BP_FirstPersonCharacter.BP_FirstPersonCharacter_C|GetHandHoldPoint _player))
  (bind _bpc_inv_belt (Variables|/Game/FirstPerson/Blueprints/BP_FirstPersonCharacter.BP_FirstPersonCharacter_C|GetBPC_Inv_Belt _player_2))
  (bind _item_details (Default|GetSlot _bpc_inv_belt New%20Slot))
  (bind (_enumname _name _description _2dimage _blueprint) (Utilities|Struct|BreakS_Item _item_details))
  (if (== New%20Slot (Variables|Default|GetActive%20Slot))
    (Development|PrintText "Swapping to same slot")
    (else
      (Variables|Default|SetActive%20Slot New%20Slot)
      (bind _helditem (Variables|Default|GetHeldItem)
        (:then
          (Actor|DestroyActor _helditem)
          (Variables|Default|SetHeldItem 0))
        (:else
          _))
      (if (Utilities|Enum|Equal(Enum) _enumname "NewEnumerator0")
        (Development|PrintText "The new slot is empty")
        (else
          (bind _returnvalue (Game|SpawnActorfromClass _blueprint (Transformation|GetRelativeTransform _handholdpoint) "Undefined" "MultiplyWithRoot" 0 0))
          (bind _output_get (Variables|Default|SetHeldItem _returnvalue))
          (Transformation|AttachComponentToComponent _output_get _handholdpoint "None" "SnapToTarget" "SnapToTarget" "KeepRelative" true)
          (Class|BPIItem|Pickup(Message) (Variables|Default|GetHeldItem) self)
          (Development|PrintText "We've spawned in the new item"))))))

(event Custom|Drop
  (bind _player (Variables|Default|GetPlayer))
  (bind _helditem (Variables|Default|GetHeldItem)
    (:then
      (Transformation|DetachFromActor (Variables|Default|GetHeldItem) "KeepWorld" "KeepWorld" "KeepWorld")
      (Class|BPIItem|Drop(Message) _helditem)
      (Variables|Default|SetHeldItem 0)
      (Default|SetSlot (Variables|/Game/FirstPerson/Blueprints/BP_FirstPersonCharacter.BP_FirstPersonCharacter_C|GetBPC_Inv_Belt _player) "NewEnumerator0" (Variables|Default|GetActive%20Slot))
      (Default|RefreshGrid (Variables|/Game/UI/W_Belt.W_Belt_C|GetW_InventoryGrid_0 (Variables|/Game/FirstPerson/Blueprints/BP_FirstPersonCharacter.BP_FirstPersonCharacter_C|GetBelt%20Widget _player))))
    (:else
      (Development|PrintText "We aren't holding anything" true true "(R=1.000000,G=0.108012,B=0.681255,A=1.000000)"))))

(event Custom|Use
  (bind _helditem (Variables|Default|GetHeldItem)
    (:then
      (Class|BPIItem|Use(Message) _helditem))
    (:else
      (Development|PrintText "We aren't holding anything" true true "(R=1.000000,G=0.108012,B=0.681255,A=1.000000)"))))

(event Custom|AltUse
  (bind _helditem (Variables|Default|GetHeldItem)
    (:then
      (Class|BPIItem|AltUse(Message) _helditem))
    (:else
      (Development|PrintText "We aren't holding anything" true true "(R=1.000000,G=0.108012,B=0.681255,A=1.000000)"))))

(event Custom|OnSlotUpdated_Event
  (params (UpdatedSlotIndex :type Integer))
  (CallFunction|UpdateHeldItem UpdatedSlotIndex))

(event Custom|UpdateHeldItem
  (params (NewChangedSlot :type Integer))
  (bind _player (Variables|Default|GetPlayer))
  (bind _handholdpoint (Variables|/Game/FirstPerson/Blueprints/BP_FirstPersonCharacter.BP_FirstPersonCharacter_C|GetHandHoldPoint _player))
  (if (== (Variables|Default|GetActive%20Slot) NewChangedSlot)
    (bind _helditem (Variables|Default|GetHeldItem)
      (:then
        (Actor|DestroyActor _helditem)
        (Variables|Default|SetHeldItem 0))
      (:else
        _))
    (if (Utilities|Enum|Equal(Enum) (.EnumName (Utilities|Struct|BreakS_Item (Default|GetSlot (Variables|/Game/FirstPerson/Blueprints/BP_FirstPersonCharacter.BP_FirstPersonCharacter_C|GetBPC_Inv_Belt (Variables|Default|GetPlayer)) (stale Custom|SwapItem New%20Slot)))) "NewEnumerator0")
      (Development|PrintText "The new slot is empty")
      (else
        (bind _returnvalue (Game|SpawnActorfromClass (.Blueprint (Utilities|Struct|BreakS_Item (Default|GetSlot (Variables|/Game/FirstPerson/Blueprints/BP_FirstPersonCharacter.BP_FirstPersonCharacter_C|GetBPC_Inv_Belt (Variables|Default|GetPlayer)) (stale Custom|SwapItem New%20Slot)))) (Transformation|GetRelativeTransform _handholdpoint) "Undefined" "MultiplyWithRoot" 0 0))
        (bind _output_get (Variables|Default|SetHeldItem _returnvalue))
        (Transformation|AttachComponentToComponent _output_get _handholdpoint "None" "SnapToTarget" "SnapToTarget" "KeepRelative" true)
        (Class|BPIItem|Pickup(Message) (Variables|Default|GetHeldItem) self)
        (Development|PrintText "We've spawned in the new item")))))

(event EventBeginPlay
  (bind _asbp_first_person_character (Utilities|Casting|CastToBP_FirstPersonCharacter (Components|GetOwner)))
  (Variables|Default|SetPlayer _asbp_first_person_character)
  (Variables|Default|SetFirst%20Person%20Camera (Variables|/Game/FirstPerson/Blueprints/BP_FirstPersonCharacter.BP_FirstPersonCharacter_C|GetFirstPersonCamera _asbp_first_person_character))
  (CallFunction|Looking)
  (CallFunction|SwapItem)
  (EventDispatchers|AssignOnSlotUpdated (Variables|/Game/FirstPerson/Blueprints/BP_FirstPersonCharacter.BP_FirstPersonCharacter_C|GetBPC_Inv_Belt (Variables|Default|GetPlayer)) (delegate Custom|OnSlotUpdated_Event)))

(event Input|KeyboardEvents|1
  (params (Key :type Key%20Structure :default "None"))
  (:Pressed
    (CallFunction|SwapItem)))

(event Input|KeyboardEvents|E
  (params (Key :type Key%20Structure :default "None"))
  (:Pressed
    (CallFunction|PickUp)))

(event Input|MouseEvents|RightMouseButton
  (params (Key :type Key%20Structure :default "None"))
  (:Pressed
    (CallFunction|AltUse)))

(event Input|KeyboardEvents|Q
  (params (Key :type Key%20Structure :default "None"))
  (:Pressed
    (CallFunction|Drop)))

(event Input|MouseEvents|LeftMouseButton
  (params (Key :type Key%20Structure :default "None"))
  (:Pressed
    (CallFunction|Use)))

(event Input|KeyboardEvents|2
  (params (Key :type Key%20Structure :default "None"))
  (:Pressed
    (CallFunction|SwapItem 1)))

(event Input|KeyboardEvents|3
  (params (Key :type Key%20Structure :default "None"))
  (:Pressed
    (CallFunction|SwapItem 2)))