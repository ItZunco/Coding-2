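; Game mode that saves and restores player inventory and per-level state through SG_Player and SG_LevelState save objects.
; BeginPlay loads existing saves or creates new objects.
; Load restores belt and backpack, activates level actors and repositions the player.
; Save writes level state under the level name alone, whereas loading and DeleteSave use a concatenated name; DeleteSave then opens the level named by SlotName.
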(event EventBeginPlay
  (Development|PrintText "Starting \"GM_SaveLoad\"" true true "(R=1.000000,G=0.243499,B=0.000000,A=1.000000)" 5.0)
  (Utilities|FlowControl|Sequence
    (:then_0
      (bind _returnvalue (SaveGame|DoesSaveGameExist (Variables|Default|GetSlot%20Name)))
      (if _returnvalue
        (CallFunction|Load)
        (Development|PrintText "Called Load")
        (else
          (bind _returnvalue_2 (SaveGame|CreateSaveGameObject "/Game/Blueprints/SaveLoad/SG_Player.SG_Player_C"))
          (Variables|Default|SetPlayerSave _returnvalue_2)
          (Development|PrintText "Created Save File"))))
    (:then_1
      (bind _returnvalue_3 (Game|GetCurrentLevelName true))
      (bind _returnvalue_4 (SaveGame|DoesSaveGameExist (Utilities|String|Append _returnvalue_3 "Default_FirstMap" (Variables|Default|GetSlot%20Name))))
      (if _returnvalue_4
        (CallFunction|Load)
        (else
          (bind _returnvalue_5 (SaveGame|CreateSaveGameObject "/Game/Blueprints/SaveLoad/SG_LevelState.SG_LevelState_C"))
          (Variables|Default|SetLevel%20State _returnvalue_5))))))

(fn ConstructionScript)

(fn Save
  (params (Belt :type Array%20of%20E_Item%20Enums :default "NewEnumerator0") (PlayerInv :type Array%20of%20E_Item%20Enums :default "NewEnumerator0") (Location :type Transform))
  (bind _playersave (Variables|Default|GetPlayerSave))
  (Utilities|FlowControl|Sequence
    (:then_0
      (Variables|/Game/Blueprints/SaveLoad/SG_Player.SG_Player_C|SetBelt _playersave Belt)
      (Variables|/Game/Blueprints/SaveLoad/SG_Player.SG_Player_C|SetPlayerInv _playersave PlayerInv)
      (SaveGame|SaveGametoSlot _playersave (Variables|Default|GetSlot%20Name)))
    (:then_1
      (Variables|/Game/Blueprints/SaveLoad/SG_LevelState.SG_LevelState_C|SetPlayerTransform (Variables|Default|GetLevel%20State) Location)
      (bind _returnvalue (Game|GetCurrentLevelName true))
      (SaveGame|SaveGametoSlot (Variables|Default|GetLevel%20State) _returnvalue))))

(fn Load
  (Utilities|FlowControl|Sequence
    (:then_0
      (bind _returnvalue (SaveGame|LoadGamefromSlot (Variables|Default|GetSlot%20Name)))
      (bind _assg_player (Utilities|Casting|CastToSG_Player _returnvalue))
      (Variables|Default|SetPlayerSave _assg_player)
      (bind _asbp_first_person_character (Utilities|Casting|CastToBP_FirstPersonCharacter (Game|GetPlayerCharacter 0))
        (:then
          (Default|SetEnumArray (Variables|/Game/FirstPerson/Blueprints/BP_FirstPersonCharacter.BP_FirstPersonCharacter_C|GetBPC_Inv_Belt _asbp_first_person_character) (Variables|/Game/Blueprints/SaveLoad/SG_Player.SG_Player_C|GetBelt (Variables|Default|GetPlayerSave)))
          (Default|SetEnumArray (Variables|/Game/FirstPerson/Blueprints/BP_FirstPersonCharacter.BP_FirstPersonCharacter_C|GetBPC_Inv_Backpack _asbp_first_person_character) (Variables|/Game/Blueprints/SaveLoad/SG_Player.SG_Player_C|GetPlayerInv (Variables|Default|GetPlayerSave)))
          (Development|PrintText "Inventory Updated"))
        (:CastFailed
          (Development|PrintText "Cast failed"))))
    (:then_1
      (bind _returnvalue_2 (Game|GetCurrentLevelName true))
      (bind _returnvalue_3 (SaveGame|LoadGamefromSlot (Utilities|String|Append _returnvalue_2 "Default_FirstMap" (Variables|Default|GetSlot%20Name))))
      (bind _assg_level_state (Utilities|Casting|CastToSG_LevelState _returnvalue_3))
      (bind _output_get (Variables|Default|SetLevel%20State _assg_level_state))
      (Default|ActivateActors _output_get)
      (bind _asbp_first_person_character_2 (Utilities|Casting|CastToBP_FirstPersonCharacter (Game|GetPlayerCharacter 0)))
      (Default|LoadTransform _asbp_first_person_character_2 (Variables|/Game/Blueprints/SaveLoad/SG_LevelState.SG_LevelState_C|GetPlayerTransform (Variables|Default|GetLevel%20State)) "0, 0, 0")
      (Pawn|SetControlRotation (Game|GetPlayerController 0) (.Rotation (Math|Transform|BreakTransform (Variables|/Game/Blueprints/SaveLoad/SG_LevelState.SG_LevelState_C|GetPlayerTransform (Variables|Default|GetLevel%20State))))))))

(fn DeleteSave
  (bind _slot_name (Variables|Default|GetSlot%20Name))
  (bind _returnvalue (Game|GetCurrentLevelName true))
  (SaveGame|DeleteGameinSlot (Utilities|String|Append _returnvalue "Default_FirstMap" _slot_name))
  (Game|OpenLevel(byName) (Utilities|String|StringToName _slot_name)))