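; SG_LevelState is a level-state object, apparently for save/load, that records activated actors and inventories.
; AddActor and AddInventory append unique entries to their lists.
; ActivateActors replays the state by calling ActivateMessage on each stored actor, then prints a debug message.
; LoadInventories is an empty stub, and an unconnected loop over the InvActors map never runs.
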(event Custom|AddActor
  (params (Actor :type Actor%20Object%20Reference%20%28by%20ref%29))
  (Utilities|Array|AddUnique (Variables|Default|GetActivatedActors) Actor))

(event Custom|ActivateActors
  (for _array_element (Variables|Default|GetActivatedActors)
    (Class|BPIActivatable|Activate(Message) _array_element))
  (Development|PrintText 0 "Activate all actors"))

(event Custom|AddInventory
  (params (Inventory :type BPC%20Inventory%20Object%20Reference%20%28by%20ref%29))
  (Utilities|Array|AddUnique (Variables|Default|GetInventories) Inventory))

(event Custom|LoadInventories)