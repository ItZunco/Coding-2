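; BP_Blaster is a blaster item that can be picked up, used and dropped.
; Pickup turns off the static mesh's collision and returns the item type, without attaching to the owner or changing physics.
; Drop restores collision, enables physics and launches the mesh along its forward vector with a mass-independent impulse.
; Use is a placeholder that only prints "Zap!", with no firing logic.
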(event EventUse
  (Development|PrintText "Zap!"))

(event EventDrop
  (bind _staticmesh (Variables|Default|GetStaticMesh))
  (Collision|SetCollisionEnabled _staticmesh "QueryAndPhysics")
  (Physics|SetSimulatePhysics _staticmesh true)
  (Physics|AddImpulse _staticmesh (* (Math|Vector|GetForwardVector _staticmesh) 1e+03) "None" true))

(fn ConstructionScript)

(fn Pickup
  (params (Owner :type BPC%20Interact%20Object%20Reference%20%28by%20ref%29))
  (Collision|SetCollisionEnabled (Variables|Default|GetStaticMesh) "NoCollision")
  (return (Variables|Default|GetItemType)))